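; Player character Blueprint with single-axis movement, jumping, sprinting, health and stamina stats, and a toggleable inventory screen.
; BeginPlay creates the HUD and inventory widgets and fills both stats.
; Tick pushes health, stamina and velocity to the HUD and handles sprinting, draining or regenerating stamina at one shared per-frame rate, unscaled by delta time.
; Jumping costs stamina, and starting a sprint requires a minimum amount and CanJump.
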(event `self.ReceiveBeginPlay`
  (`self.Interface Widgets`)
  (`self.Init Stats`))

(event `self.ReceiveTick`
  (params (DeltaSeconds :type "Float (single-precision)"))
  (`self.Update Health Bar`)
  (`self.Handle Sprint`)
  (`self.Update Stamina`)
  (`self.Display Speed`))

(event `InputAxis|MoveX`
  (params (AxisValue :type "Float (single-precision)"))
  (`self.AddMovementInput` (`SceneComponent.GetForwardVector` (`self.CapsuleComponent`)) (`self.GetInputAxisValue`)))

(event `InputAction|Jump`
  (params (Key :type "Key Structure"))
  (:`Pressed`
    (if (and (`self.CanJump`) (> (`self.Stamina`) (`self.Jump Exhaust Rate`)))
      (`self.Jump`)
      (set `self.Stamina` (- (`self.Stamina`) (`self.Jump Exhaust Rate`))))))

(event `InputAction|Sprint`
  (params (Key :type "Key Structure"))
  (:`Pressed`
    (if (`self.CanJump`)
      (if (> (`self.Stamina`) (`self.Minimum Stamina`))
        (set `self.Sprint` true))
      (else
        (set `self.Sprint` false :!label _label)
        (set `CharacterMovementComponent.MaxWalkSpeed` (`self.Walk Speed`) (`self.CharacterMovement`)))))
  (:`Released`
    (goto _label)))

(event `InputAction|Inventory`
  (params (Key :type "Key Structure"))
  (:`Pressed`
    (`self.Open/Close Inventory`)))

(fn `Display Speed`
  (`EditableText.SetText` (`/Game/Blueprints/Player/UI.CurrentSpeed` (`self.UserInterface`)) (`KismetTextLibrary.Conv_VectorToText` (`CharacterMovementComponent.GetLastUpdateVelocity` (`self.CharacterMovement`)))))

(fn `Handle Sprint`
  (if (`self.Sprint`)
    (if (> (`self.Stamina`) 0.0)
      (if (`self.CanJump`)
        (set `self.Stamina` (- (`self.Stamina`) (`self.Sprint Exhaust Rate`)))
        (set `CharacterMovementComponent.MaxWalkSpeed` (`self.Sprint Speed`) (`self.CharacterMovement`)))
      (else
        (set `self.Sprint` false)
        (set `self.Stamina` 0.0)
        (set `CharacterMovementComponent.MaxWalkSpeed` (`self.Walk Speed`) (`self.CharacterMovement`))))
    (elif (< (`self.Stamina`) (`self.Max Stamina`))
      (set `self.Stamina` (+ (`self.Stamina`) (`self.Sprint Exhaust Rate`)))
      (else
        (set `self.Stamina` (`self.Max Stamina`))))))

(fn `Init Stats`
  (set `self.Health` (`self.Max Health`))
  (set `self.Stamina` (`self.Max Stamina`)))

(fn `Interface Widgets`
  (bind _returnvalue (`|CreateWidget` "/Game/Blueprints/Player/UI.UI_C"))
  (set `self.UserInterface` _returnvalue)
  (bind _returnvalue_2 (`|CreateWidget` "/Game/Blueprints/Player/Inventory.Inventory_C"))
  (set `self.Inventory` _returnvalue_2)
  (`UserWidget.AddToViewport` (`self.UserInterface`) 0))

(fn `Open/Close Inventory`
  (bind _inventory (`self.Inventory`))
  (if (`self.Inventory_Open`)
    (set `self.Inventory_Open` false)
    (`Widget.RemoveFromParent` _inventory)
    (else
      (set `self.Inventory_Open` true)
      (`UserWidget.AddToViewport` _inventory 0))))

(fn `Update Health Bar`
  (`ProgressBar.SetPercent` (`/Game/Blueprints/Player/UI.Health` (`self.UserInterface`)) (/ (`self.Health`) (`self.Max Health`))))

(fn `Update Stamina`
  (`ProgressBar.SetPercent` (`/Game/Blueprints/Player/UI.Stamina` (`self.UserInterface`)) (/ (`self.Stamina`) (`self.Max Stamina`))))

(fn `UserConstructionScript`)